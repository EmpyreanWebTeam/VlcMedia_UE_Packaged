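; TV actor that plays video with sound on a screen mesh through a Media Player.
; BeginPlay links the media sound, builds a dynamic screen material with video texture, brightness and rotation, then optionally autoplays.
; Playback opens the clamped start channel from MediaList, or SourceUrl unchecked if the list is empty, and starts when media opens.
; NextChannel and PrevChannel step the list index by modulo, which goes negative when stepping back from zero.
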(event `self.ReceiveBeginPlay`
  (bind _mediaplayer (`self.MediaPlayer`))
  (`self.EnableInput` (`GameplayStatics.GetPlayerController` 0))
  (`MediaSoundComponent.SetMediaPlayer` (`self.MediaSound`) _mediaplayer)
  (`self.SetupMaterial`)
  (`KismetSystemLibrary.Delay` 0.1)
  (add `MediaPlayer.OnMediaOpened` _mediaplayer (delegate `OnMediaOpened_Event`))
  (if (`self.AutoPlayOnBegin`)
    (`self.PlayByListOrUrl`)))

(event `OnMediaOpened_Event`
  (params (OpenedUrl :type String))
  (`MediaPlayer.Play` (`self.MediaPlayer`)))

(fn `NextChannel`
  (bind _mediaplayer (`self.MediaPlayer`))
  (bind _returnvalue (`KismetArrayLibrary.Array_Length` (`self.MediaList`)))
  (if (> _returnvalue 0)
    (bind _output_get (set `self.ChannelIndex` (mod (+ (`self.ChannelIndex`) 1) _returnvalue)))
    (`MediaPlayer.Close` _mediaplayer)
    (`MediaPlayer.OpenSource` _mediaplayer (`|GetArrayItem` (`self.MediaList`) _output_get))))

(fn `PlayByListOrUrl`
  (bind _returnvalue (`KismetArrayLibrary.Array_Length` (`self.MediaList`)))
  (if (> _returnvalue 0)
    (bind _output_get (set `self.ChannelIndex` (`KismetMathLibrary.Clamp` (`self.StartChannel`) 0 (- _returnvalue 1))))
    (`MediaPlayer.Close` (`self.MediaPlayer`))
    (`MediaPlayer.OpenSource` (`self.MediaPlayer`) (`|GetArrayItem` (`self.MediaList`) _output_get))
    (elif true
      (`MediaPlayer.Close` (`self.MediaPlayer`))
      (`MediaPlayer.OpenUrl` (`self.MediaPlayer`) (`self.SourceUrl`))
      (else
        (`KismetSystemLibrary.PrintString` "No MediaList and SourceUrl is empty.")))))

(fn `PrevChannel`
  (bind _mediaplayer (`self.MediaPlayer`))
  (bind _returnvalue (`KismetArrayLibrary.Array_Length` (`self.MediaList`)))
  (if (> _returnvalue 0)
    (bind _output_get (set `self.ChannelIndex` (mod (- (`self.ChannelIndex`) 1) _returnvalue)))
    (`MediaPlayer.Close` _mediaplayer)
    (`MediaPlayer.OpenSource` _mediaplayer (`|GetArrayItem` (`self.MediaList`) _output_get))))

(fn `SetupMaterial`
  (bind _dmi (`self.DMI`))
  (bind _returnvalue (`PrimitiveComponent.CreateDynamicMaterialInstance` (`self.Screen`) 0 null "None"))
  (set `self.DMI` _returnvalue)
  (`MaterialInstanceDynamic.SetTextureParameterValue` _dmi "VideoTex" (`self.MediaTexture`))
  (`MaterialInstanceDynamic.SetScalarParameterValue` _dmi "EmissiveIntensity" (`self.Brightness`))
  (`MaterialInstanceDynamic.SetScalarParameterValue` _dmi "Rotation" (`self.Rotation`)))

(fn `UserConstructionScript`)